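; Session manager for LAN multiplayer on Magic Leap (Lumin) that lets input actions host or join a game.
; Start opens DefaultServerMap as a listen server and Find connects to a hardcoded localhost address, both gated by EnsureNetworkPrivileges, which checks or requests LAN privilege on Lumin only.
; BeginPlay enables input and configures hand gesture recognition.
; Find and create session logic exists but is disconnected and never runs.
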(event EventBeginPlay
  (Input|EnableInput (Game|GetPlayerController 0))
  (Class|MagicLeapHandTrackingFunctionLibrary|SetConfiguration (Variables|Default|GetGesturesToEnable) "SimpleSmoothing" "SlightRobustnessToFlicker" true))

(event Input|ActionEvents|InputActionFindGameSessions
  (params (Key :type Key%20Structure :default "None"))
  (:Pressed
    (bind _bgranted (CallFunction|EnsureNetworkPrivileges))
    (if _bgranted
      (Game|OpenLevel(byName) "127.0.0.1:7777")
      (else
        (Development|PrintString "LAN priv not granted. What are we even doing here")))))

(event Input|ActionEvents|InputActionStartGameSession
  (params (Key :type Key%20Structure :default "None"))
  (:Pressed
    (bind _bgranted (CallFunction|EnsureNetworkPrivileges))
    (if _bgranted
      (Game|OpenLevel(byName) "DefaultServerMap?Listen")
      (else
        (Development|PrintString "LAN priv not granted. What are we even doing here")))))

(fn ConstructionScript)

(fn EnsureNetworkPrivileges
  (if (Utilities|Enum|Equal(Enum) (Game|GetPlatformName) "Lumin")
    (bind _returnvalue (Class|MagicLeapPrivilegesFunctionLibrary|CheckPrivilege "LocalAreaNetwork"))
    (if _returnvalue
      _
      (else
        (bind _returnvalue_2 (Class|MagicLeapPrivilegesFunctionLibrary|RequestPrivilege "LocalAreaNetwork"))
        (return _returnvalue_2))))
  (return true))