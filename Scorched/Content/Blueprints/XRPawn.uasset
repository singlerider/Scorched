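; XR pawn that works with a headset or as a desktop free-fly pawn, replicating its view to other players.
; Axis inputs drive FloatingPawnMovement and controller rotation, with pawn pitch/yaw following the controller when no HMD is connected.
; Each tick the owning client sends the XRCamera relative transform (HMD) or XRCameraRoot world transform (desktop) through server-to-multicast RPCs.
; Receivers apply these as relative transforms, skipping the owning client via HasLocalNetOwner.
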(event Custom|Multicast_SetCameraTransform
  (params (NewTransform :type Transform%20%28by%20ref%29))
  ;[1 1 1] Pawn Camera Transform Replication
  (Networking|SwitchHasAuthority
    (:Authority
      (Transformation|SetRelativeTransform (Variables|Default|GetXRCamera) NewTransform false false :!label _label))
    (:Remote
      (if (not (CallFunction|HasLocalNetOwner))
        (goto _label)))))

(event Custom|Server_SetCameraTransform
  (params (NewTransform :type Transform%20%28by%20ref%29))
  ;[1 1 1] Pawn Camera Transform Replication
  (CallFunction|MulticastSetCameraTransform NewTransform))

(event Custom|Server_SetCameraRootTransform
  (params (NewLocation :type Vector) (NewRotation :type Rotator))
  ;[1 1 1] Pawn Camera Root Transform Replication
  (CallFunction|MulticastSetCameraRootTransform NewLocation NewRotation))

(event Custom|Multicast_SetCameraRootTransform
  (params (NewLocation :type Vector) (NewRotation :type Rotator))
  ;[1 1 1] Pawn Camera Root Transform Replication
  (Networking|SwitchHasAuthority
    (:Authority
      (Transformation|SetRelativeLocationAndRotation (Variables|Default|GetXRCameraRoot) NewLocation NewRotation false false :!label _label))
    (:Remote
      (if (not (CallFunction|HasLocalNetOwner))
        (goto _label)))))

(event EventBeginPlay
  (if (not (Class|HeadMountedDisplayFunctionLibrary|IsHeadMountedDisplayConnected))
    (Variables|Default|SetbUseControllerRotationPitch true)
    (Variables|Default|SetbUseControllerRotationYaw true)))

(event EventTick
  (params (DeltaSeconds :type Float%20%28single-precision%29))
  (bind _xrcameraroot (Variables|Default|GetXRCameraRoot))
  (|CallParentFunction DeltaSeconds)
  (if (not (Class|HeadMountedDisplayFunctionLibrary|IsHeadMountedDisplayConnected))
    ;[1 1 1] Replicate XRCameraRoot transform if running without HMD
    (Networking|SwitchHasAuthority
      (:Remote
        (if (CallFunction|HasLocalNetOwner)
          (CallFunction|ServerSetCameraRootTransform (Transformation|GetWorldLocation _xrcameraroot) (Transformation|GetWorldRotation _xrcameraroot)))))
    (else
      ;[1 1 1] Replicate pawn camera transform
      (Networking|SwitchHasAuthority
        (:Remote
          (if (CallFunction|HasLocalNetOwner)
            (CallFunction|ServerSetCameraTransform (Transformation|GetRelativeTransform (Variables|Default|GetXRCamera)))))))))

(event Input|AxisEvents|InputAxisMoveForward
  (params (AxisValue :type Float%20%28single-precision%29))
  ;[1 1 1] Movement stuff from DefaultPawn, used only on Desktop
  (Class|PawnMovementComponent|AddInputVector (Variables|Default|GetFloatingPawnMovement) (* (Math|Vector|GetForwardVector (Variables|Default|GetXRCamera)) AxisValue) false))

(event Input|AxisEvents|InputAxisMoveRight
  (params (AxisValue :type Float%20%28single-precision%29))
  ;[1 1 1] Movement stuff from DefaultPawn, used only on Desktop
  (Class|PawnMovementComponent|AddInputVector (Variables|Default|GetFloatingPawnMovement) (* (Math|Vector|GetRightVector (Variables|Default|GetXRCamera)) AxisValue) false))

(event Input|AxisEvents|InputAxisMoveUp
  (params (AxisValue :type Float%20%28single-precision%29))
  ;[1 1 1] Movement stuff from DefaultPawn, used only on Desktop
  (Class|PawnMovementComponent|AddInputVector (Variables|Default|GetFloatingPawnMovement) (* (Math|Vector|GetUpVector (Variables|Default|GetXRCamera)) AxisValue) false))

(event Input|AxisEvents|InputAxisTurnRate
  (params (AxisValue :type Float%20%28single-precision%29))
  ;[1 1 1] Movement stuff from DefaultPawn, used only on Desktop
  (Pawn|Input|AddControllerYawInput (* (* AxisValue 45.0) (Utilities|Time|GetWorldDeltaSeconds))))

(event Input|AxisEvents|InputAxisLookUp
  (params (AxisValue :type Float%20%28single-precision%29))
  ;[1 1 1] Movement stuff from DefaultPawn, used only on Desktop
  (Pawn|Input|AddControllerPitchInput (* (* AxisValue 45.0) (Utilities|Time|GetWorldDeltaSeconds))))

(fn ConstructionScript)

(fn HasLocalNetOwner
  (LocalVariables|SetTopOwner self)
  (while (Utilities|IsValid (Components|GetOwner (LocalVariables|GetTopOwner)))
    (LocalVariables|SetTopOwner 0))
  (bind _aspawn (Utilities|Casting|CastToPawn (LocalVariables|GetTopOwner))
    (:then
      (return (Pawn|IsLocallyControlled _aspawn)))
    (:CastFailed
      (bind _ascontroller (Utilities|Casting|CastToController (LocalVariables|GetTopOwner))
        (:then
          (return (Pawn|IsLocalController _ascontroller)))
        (:CastFailed
          (return false))))))